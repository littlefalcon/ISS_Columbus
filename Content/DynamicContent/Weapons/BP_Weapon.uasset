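; Base weapon Blueprint that tracks battery-style magazine ammo and overheat.
; BeginPlay fills the magazine, converts the fire rate and scales down battery use for one weapon type, while Tick steadily cools heat.
; DeceaseClip either just checks ammo or spends battery and adds heat, returning false on depletion or overheat.
; Fire, AssignProjectile and DeceaseMagazine events are empty, and the muzzle sound code is disconnected.
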(event `self.ReceiveTick`
  (params (DeltaSeconds :type "Float (single-precision)"))
  (if (> (`self.CurrentOverheat`) 0.0)
    (set `self.CurrentOverheat` (- (`self.CurrentOverheat`) (* DeltaSeconds 10.0)))))

(event `self.ReceiveBeginPlay`
  (`self.SetupWeapon`))

(event `Fire`)

(event `AssignProjectile`)

(event `DeceaseMagazine`)

(fn `ConvertFireRate`
  (bind _output_get (set `self.FireRate` (`/Game/DynamicContent/Engine/GlobalMacros.ConvertFirerate` (`self.FireRate`))))
  (`/Game/DynamicContent/Engine/GlobalMacros.SpeedDebug` (`KismetStringLibrary.Conv_DoubleToString` _output_get))
  (return))

(fn `DeceaseClip`
  (params (CheckAmmo :type Boolean))
  (returns (IsHaveAmmo :type Boolean))
  (bind _returnvalue (`self.OverheatResult`))
  (bind _currentmagazinecapacity (`self.CurrentMagazineCapacity`))
  ;[1 1 1] Check or Fire Ammo
  (if CheckAmmo
    (`self.CheckAmmo`
      (:`Have`
        _)
      (:`Deplete`
        (return false)))
    (else
      ;[1 1 1] Overheat Condition Check
      (if (>= _returnvalue (`self.MaxOverheat`))
        (return false)
        (else
          (bind _output_get (set `self.CurrentOverheat` _returnvalue))
          ;[1 1 1] Decease Ammo Condition Check
          (if (> _currentmagazinecapacity 0.0)
            (bind _output_get_2 (set `self.CurrentMagazineCapacity` (- _currentmagazinecapacity (`self.BatteryConsume`))))
            (`/Game/DynamicContent/Engine/GlobalMacros.FastDebug` (`KismetStringLibrary.Conv_DoubleToString` _output_get_2) "  < Current Ammo | Heat >  " (`KismetStringLibrary.Conv_DoubleToString` _output_get))
            ;[1 1 1] IS OVERHEAT?
            (if (>= (`self.CurrentOverheat`) (`self.MaxOverheat`))
              (return false)
              (else
                _))
            (else
              (bind _output_get_3 (set `self.CurrentMagazineCapacity` 0.0))
              (`/Game/DynamicContent/Engine/GlobalMacros.FastDebug` "AMMO DEPLETE" (`KismetStringLibrary.Conv_DoubleToString` _output_get_3))
              (return false)))))))
  (return true))

(fn `SetupWeapon`
  (set `self.CurrentMagazineCapacity` (`self.MagazineCapacity`))
  (`self.ConvertFireRate`)
  (if (== (`self.WeaponType`) 1)
    (bind _output_get (set `self.BatteryConsume` (/ (`self.BatteryConsume`) 10.0))))
  (`/Game/DynamicContent/Engine/GlobalMacros.FastDebug` "DAMAGE  " (`KismetStringLibrary.Conv_DoubleToString` _output_get) "<<<" (`KismetStringLibrary.Conv_DoubleToString` (`self.Damage`))))

(fn `UserConstructionScript`)