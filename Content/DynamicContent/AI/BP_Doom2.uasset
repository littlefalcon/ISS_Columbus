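; BP_Doom2 is an AI enemy Blueprint for the Doom2 creature that handles its attack animation.
; PlayAttackAnimation randomly plays one of two non-looping attack clips directly on the passed InfectedActor, then sets Attacking to true.
; After a fixed delay it switches its own Mesh back to Animation Blueprint mode, if valid, and does not clear Attacking here.
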(event `self.PlayAttackAnimation`
  (params (InfectedActor :type "SkeletalMeshComponent Object Reference") (NewAnimToPlay :type "AnimationAsset Object Reference"))
  (bind _mesh (`self.Mesh`))
  (switch `int` (`KismetMathLibrary.RandomInteger` 2)
    (:`Default`
      (`SkeletalMeshComponent.PlayAnimation` InfectedActor "/Game/DynamicContent/AI/DoomRigged/Doom2Rigged_Anim_rig_doom2_atk.Doom2Rigged_Anim_rig_doom2_atk" false :!label _label))
    (:`0`
      (goto _label))
    (:`1`
      (`SkeletalMeshComponent.PlayAnimation` InfectedActor "/Game/DynamicContent/AI/DoomRigged/Doom2Rigged_Anim_rig_doom2_atk_2.Doom2Rigged_Anim_rig_doom2_atk_2" false)))
  (set `self.Attacking` true)
  (`KismetSystemLibrary.Delay` 1.5)
  (`/Engine/EditorBlueprintResources/StandardMacros.IsValid` _mesh
    (:`Is Valid`
      (`SkeletalMeshComponent.SetAnimationMode` _mesh "AnimationBlueprint"))))

(fn `UserConstructionScript`
  (`parent.UserConstructionScript`))