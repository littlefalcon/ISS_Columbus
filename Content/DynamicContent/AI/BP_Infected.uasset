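; BP_Infected is an AI enemy character with Walk, Run and melee Attack events, damaging the player through a weapon overlap.
; Socket-attached body-part colliders feed projectile overlaps into HitResponse, which applies location-based damage, plays a reaction and flags the Blackboard.
; PawnSensing passes heard noise locations to the Blackboard, while its sight event is empty.
; Death spawns effects, random items and GameManager-selected craft drops, then destroys the actor and reports the kill.
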(event `self.Col_Head.OnComponentBeginOverlap`
  (params (OverlappedComponent :type "PrimitiveComponent Object Reference") (OtherActor :type "Actor Object Reference") (OtherComp :type "PrimitiveComponent Object Reference") (OtherBodyIndex :type Integer) (bFromSweep :type Boolean) (SweepResult :type "HitResult Structure (by ref)"))
  ;[1 1 1] Hit Mechanic
  (`self.HitResponse` (`self.Mesh`) (`self.CapsuleComponent`) OtherActor 2.0 "HEAD"))

(event `self.Col_LL.OnComponentBeginOverlap`
  (params (OverlappedComponent :type "PrimitiveComponent Object Reference") (OtherActor :type "Actor Object Reference") (OtherComp :type "PrimitiveComponent Object Reference") (OtherBodyIndex :type Integer) (bFromSweep :type Boolean) (SweepResult :type "HitResult Structure (by ref)"))
  ;[1 1 1] Hit Mechanic
  (`self.HitResponse` (`self.Mesh`) (`self.CapsuleComponent`) OtherActor 0.75 "LL"))

(event `self.Col_RL.OnComponentBeginOverlap`
  (params (OverlappedComponent :type "PrimitiveComponent Object Reference") (OtherActor :type "Actor Object Reference") (OtherComp :type "PrimitiveComponent Object Reference") (OtherBodyIndex :type Integer) (bFromSweep :type Boolean) (SweepResult :type "HitResult Structure (by ref)"))
  ;[1 1 1] Hit Mechanic
  (`self.HitResponse` (`self.Mesh`) (`self.CapsuleComponent`) OtherActor 0.75 "LR"))

(event `self.Col_LA.OnComponentBeginOverlap`
  (params (OverlappedComponent :type "PrimitiveComponent Object Reference") (OtherActor :type "Actor Object Reference") (OtherComp :type "PrimitiveComponent Object Reference") (OtherBodyIndex :type Integer) (bFromSweep :type Boolean) (SweepResult :type "HitResult Structure (by ref)"))
  ;[1 1 1] Hit Mechanic
  (`self.HitResponse` (`self.Mesh`) (`self.CapsuleComponent`) OtherActor 1.5 "LA"))

(event `self.Col_RA.OnComponentBeginOverlap`
  (params (OverlappedComponent :type "PrimitiveComponent Object Reference") (OtherActor :type "Actor Object Reference") (OtherComp :type "PrimitiveComponent Object Reference") (OtherBodyIndex :type Integer) (bFromSweep :type Boolean) (SweepResult :type "HitResult Structure (by ref)"))
  ;[1 1 1] Hit Mechanic
  (`self.HitResponse` (`self.Mesh`) (`self.CapsuleComponent`) OtherActor 1.5 "RA"))

(event `self.Col_Body.OnComponentBeginOverlap`
  (params (OverlappedComponent :type "PrimitiveComponent Object Reference") (OtherActor :type "Actor Object Reference") (OtherComp :type "PrimitiveComponent Object Reference") (OtherBodyIndex :type Integer) (bFromSweep :type Boolean) (SweepResult :type "HitResult Structure (by ref)"))
  ;[1 1 1] Hit Mechanic
  (`self.HitResponse` (`self.Mesh`) (`self.CapsuleComponent`) OtherActor 1.0 "BODY"))

(event `Walk`
  (set `CharacterMovementComponent.MaxWalkSpeed` 200.0 (`self.CharacterMovement`)))

(event `Run`
  (set `CharacterMovementComponent.MaxWalkSpeed` 500.0 (`self.CharacterMovement`)))

(event `Attack`
  (bind _mesh (`self.Mesh`))
  (bind _mesh_2 (`self.Mesh`))
  (`/Engine/EditorBlueprintResources/StandardMacros.IsValid` _mesh
    (:`Is Valid`
      (`self.PlayAttackAnimation` _mesh "/Game/StaticContent/MixamoAnimPack/Mixamo_Alpha/Anims/mixamo_Sword_Swing.mixamo_Sword_Swing")
      (set `self.Attacking` true)
      (`KismetSystemLibrary.Delay` 1.5)
      (`/Engine/EditorBlueprintResources/StandardMacros.IsValid` _mesh_2
        (:`Is Valid`
          (`SkeletalMeshComponent.SetAnimationMode` _mesh_2 "AnimationBlueprint"))))))

(event `On Spawned`
  (`/Game/DynamicContent/AI/InfectedController.On Spawned` (stale `self.ReceiveBeginPlay` _output_get)))

(event `self.ReceiveBeginPlay`
  (bind _asinfected_controller (cast `/Game/DynamicContent/AI/InfectedController` (`AIBlueprintHelperLibrary.GetAIController` self)))
  (bind _output_get (set `self.InfectedController` _asinfected_controller)))

(event `self.WeaponCollision.OnComponentBeginOverlap`
  (params (OverlappedComponent :type "PrimitiveComponent Object Reference") (OtherActor :type "Actor Object Reference") (OtherComp :type "PrimitiveComponent Object Reference") (OtherBodyIndex :type Integer) (bFromSweep :type Boolean) (SweepResult :type "HitResult Structure (by ref)"))
  (if (`self.Attacking`)
    (bind _asbp_player (cast `/Game/DynamicContent/Player/BP_Player` OtherActor))
    (`/Game/DynamicContent/Player/BP_Player.TakeDamage` _asbp_player)
    (set `self.Attacking` false)))

(event `self.PawnSensing.OnSeePawn`
  (params (Pawn :type "Pawn Object Reference")))

(event `self.PawnSensing.OnHearNoise`
  (params (Instigator :type "Pawn Object Reference") (Location :type "Vector Structure (by ref)") (Volume :type "Float (single-precision)"))
  (bind _returnvalue (`AIBlueprintHelperLibrary.GetBlackboard` null))
  (set `self.SoundMaker` Instigator)
  (bind _output_get (set `self.SoundLocation` Location))
  (`BlackboardComponent.SetValueAsVector` _returnvalue "SoundLocation" _output_get)
  (`BlackboardComponent.SetValueAsBool` _returnvalue "IsHear" true))

(fn `GetSpawnArea`
  (returns (SpawnArea :type Name))
  (return (`self.SpawnAreaTag`)))

(fn `PlayAttackAnimation`
  (params (InfectedActor :type "SkeletalMeshComponent Object Reference") (NewAnimToPlay :type "AnimationAsset Object Reference"))
  (`SkeletalMeshComponent.PlayAnimation` InfectedActor NewAnimToPlay false)
  (`/Game/DynamicContent/Engine/GlobalMacros.FastDebug` "aaaaaa"))

(fn `UserConstructionScript`
  (bind _mesh (`self.Mesh`))
  (bind _mesh_2 (`self.Mesh`))
  (`SceneComponent.K2_AttachToComponent` (`self.Weapon`) (`self.Mesh`) (`self.HitSocket`) "KeepRelative" "KeepRelative" "KeepRelative" true)
  (`SceneComponent.K2_AttachToComponent` (`self.Col_Head`) (`self.Mesh`) "Col_Head" "KeepRelative" "KeepRelative" "KeepRelative" true)
  (`SceneComponent.K2_AttachToComponent` (`self.Col_LA`) _mesh "Col_LA" "KeepRelative" "KeepRelative" "KeepRelative" true)
  (`SceneComponent.K2_AttachToComponent` (`self.Col_RA`) _mesh "Col_RA" "KeepRelative" "KeepRelative" "KeepRelative" true)
  (`SceneComponent.K2_AttachToComponent` (`self.Col_Body`) _mesh_2 "Col_Body" "KeepRelative" "KeepRelative" "KeepRelative" true)
  (`SceneComponent.K2_AttachToComponent` (`self.Col_LL`) _mesh_2 "Col_LL" "KeepRelative" "KeepRelative" "KeepRelative" true)
  (`SceneComponent.K2_AttachToComponent` (`self.Col_RL`) (`self.Mesh`) "Col_RL" "KeepRelative" "KeepRelative" "KeepRelative" true))